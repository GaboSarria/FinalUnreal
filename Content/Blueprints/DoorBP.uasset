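; Interactive door actor that the player swings open and closed with the E key while nearby.
; Overlapping the Box component enables input for the first player controller, and ending an actor overlap disables it.
; E checks the Door_Rotation timeline value to either play it forward with a squeak sound or reverse it silently.
; The timeline's DoorRot track drives the relative yaw of the Puerta component.
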(event `self.Box.OnComponentBeginOverlap`
  (params (OverlappedComponent :type "PrimitiveComponent Object Reference") (OtherActor :type "Actor Object Reference") (OtherComp :type "PrimitiveComponent Object Reference") (OtherBodyIndex :type Integer) (bFromSweep :type Boolean) (SweepResult :type "HitResult Structure (by ref)"))
  (`self.EnableInput` (`GameplayStatics.GetPlayerController` 0)))

(event `self.ReceiveActorEndOverlap`
  (params (OtherActor :type "Actor Object Reference"))
  (`self.DisableInput` (`GameplayStatics.GetPlayerController` 0)))

(event `Key|E`
  (params (Key :type "Key Structure" :default "AnyKey"))
  (:`Pressed`
    (if (< (stale _doorrot) 1.0)
      (`GameplayStatics.PlaySound2D` "/Game/Sonidos/Ambientacion/Squeak_Cue.Squeak_Cue")
      (bind (_direction _doorrot) (`Timeline|Door_Rotation` :!label _label)
        (:`Update`
          (`SceneComponent.K2_SetRelativeRotation` (`self.Puerta`) (`KismetMathLibrary.MakeRotator` 0.0 0.0 _doorrot) false false)))
      (else
        (goto _label :!via `Reverse`)))))

(fn `UserConstructionScript`)